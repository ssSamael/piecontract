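; Game mode for a corridor level that spawns floor tile actors when play begins.
; BeginPlay runs a single-pass loop calling AddMoreTiles, which spawns one BP_Tile2 at SpawnPoint.
; AddFloorTile chains BP_Tile actors by storing each tile's attach transform as NextSpawnPoint, but its ten-tile loop is disconnected.
; The BP_Tile3 and BP_Tile4 spawns in AddMoreTiles are also unwired and never run.
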(event EventBeginPlay
  (for _index (range 0 0)
    (CallFunction|AddMoreTiles)))

(fn ConstructionScript)

(fn AddFloorTile
  (bind _returnvalue (Game|SpawnActorfromClass "/Game/Project/Blueprints/BP_Tile.BP_Tile_C" (Variables|Default|GetNextSpawnPoint) "Undefined" 0 0))
  (bind _attachtransform (Default|GetAttachTransform _returnvalue))
  (Variables|Default|SetNextSpawnPoint _attachtransform))

(fn AddMoreTiles
  (Game|SpawnActorfromClass "/Game/Project/Blueprints/BP_Tile2.BP_Tile2_C" (Variables|Default|GetSpawnPoint) "Undefined" 0 0))