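; BP_Tile4 is a moving corridor tile that scrolls along negative X and removes itself.
; Tick re-issues MoveComponentTo on the root to keep it sliding by a move distance.
; After a fixed delay from BeginPlay, it asks CorridorGameMode to add more tiles, and GetAttachTransform exposes its AttachPoint's world transform.
; When EndTrigger overlaps a Barrier, the tile destroys itself.
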(event OnComponentBeginOverlap(EndTrigger)
  (params (OverlappedComponent :type Primitive%20Component%20Object%20Reference) (OtherActor :type Actor%20Object%20Reference) (OtherComp :type Primitive%20Component%20Object%20Reference) (OtherBodyIndex :type Integer) (bFromSweep :type Boolean) (SweepResult :type Hit%20Result%20Structure%20%28by%20ref%29))
  (Utilities|Casting|CastToBarrier OtherActor)
  (Utilities|Casting|CastToCorridorGameMode (Game|GetGameMode))
  (Utilities|FlowControl|Delay 0.0)
  (Actor|DestroyActor))

(event EventBeginPlay
  (Utilities|FlowControl|Delay 3.34)
  (bind _ascorridor_game_mode (Utilities|Casting|CastToCorridorGameMode (Game|GetGameMode)))
  (Default|AddMoreTiles _ascorridor_game_mode))

(event EventTick
  (params (DeltaSeconds :type Float%20%28single-precision%29))
  (bind _defaultsceneroot (Variables|Default|GetDefaultSceneRoot))
  (bind _relativelocation (Variables|/Script/Engine.SceneComponent|GetRelativeLocation _defaultsceneroot))
  (Components|MoveComponentTo _defaultsceneroot (Math|Vector|MakeVector (- (.x _relativelocation) (Variables|Default|GetMoveDistance)) (.y _relativelocation) (.z _relativelocation)) (Variables|/Script/Engine.SceneComponent|GetRelativeRotation _defaultsceneroot) false false 2e+01 false))

(fn ConstructionScript)

(fn GetAttachTransform
  (return (Transformation|GetWorldTransform (Variables|Default|GetAttachPoint))))